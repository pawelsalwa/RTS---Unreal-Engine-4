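; BP_SalwusUnit is a selectable, team-based combat unit that spawns its own controller and an Akacz actor attached to its Hand socket.
; Sphere overlaps maintain a list of visible enemy units and choose the current target, which the unit turns to face every tick.
; Attack toggles an IsAttacking window using delays and enforces a cooldown.
; Selection shows or hides the CursorToWorld component.
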(event `HandleSelection`
  (params (Selected :type Boolean))
  (`SceneComponent.SetHiddenInGame` (`self.CursorToWorld`) (not Selected) false))

(event `self.ReceiveBeginPlay`
  (`self.SpawnDefaultController`)
  (bind _returnvalue (`|SpawnActorFromClass` "/Game/MainContent/Items/Weapons/Akacz.Akacz_C" (`KismetMathLibrary.MakeTransform` (0.0 0.0 0.0)) "Undefined" "OverrideRootScale" null null))
  (`self.K2_AttachToActor` _returnvalue self "Hand" "KeepRelative" "KeepRelative" "KeepRelative" true))

(event `self.ReceiveTick`
  (params (DeltaSeconds :type "Float (single-precision)"))
  ;[1 1 1] event tick
  (if (`self.bHasTargetToAttack`)
    (bind _output_get (set `self.TargetRotation` (`KismetMathLibrary.FindLookAtRotation` (`self.K2_GetActorLocation`) (`self.K2_GetActorLocation` (`self.UnitTargetToAttack`)))))
    (`self.K2_SetActorRotation` _output_get)))

(event `self.Sphere.OnComponentBeginOverlap`
  (params (OverlappedComponent :type "PrimitiveComponent Object Reference") (OtherActor :type "Actor Object Reference") (OtherComp :type "PrimitiveComponent Object Reference") (OtherBodyIndex :type Integer) (bFromSweep :type Boolean) (SweepResult :type "HitResult Structure (by ref)"))
  ;[1 1 1] on comp begin overlap
  (bind _asbp_salwus_unit (cast `/Game/MainContent/Blueprints/BP_SalwusUnit` OtherActor))
  (if (`|EnumInequality` (`MyCharacter.Team` _asbp_salwus_unit) (`self.Team`))
    (`KismetArrayLibrary.Array_AddUnique` (`self.VisibleUnits`) _asbp_salwus_unit)
    (if (not (`self.bHasTargetToAttack`))
      (set `self.UnitTargetToAttack` _asbp_salwus_unit)
      (set `self.bHasTargetToAttack` true))))

(event `self.Sphere.OnComponentEndOverlap`
  (params (OverlappedComponent :type "PrimitiveComponent Object Reference") (OtherActor :type "Actor Object Reference") (OtherComp :type "PrimitiveComponent Object Reference") (OtherBodyIndex :type Integer))
  ;[1 1 1] on comp end overlap
  (bind _asbp_salwus_unit (cast `/Game/MainContent/Blueprints/BP_SalwusUnit` OtherActor))
  (if (`|EnumInequality` (`MyCharacter.Team` _asbp_salwus_unit) (`self.Team`))
    (`KismetArrayLibrary.Array_RemoveItem` (`self.VisibleUnits`) _asbp_salwus_unit)
    (if (== (`KismetArrayLibrary.Array_Length` (`self.VisibleUnits`)) 0)
      (set `self.bHasTargetToAttack` false)
      (elif (== _asbp_salwus_unit (`self.UnitTargetToAttack`))
        (bind _asbp_salwus_unit_2 (cast `/Game/MainContent/Blueprints/BP_SalwusUnit` (`|GetArrayItem` (`self.VisibleUnits`))))
        (set `self.UnitTargetToAttack` _asbp_salwus_unit_2)))))

(event `self.Attack`
  (if (`self.bCanAttack`)
    (set `self.bCanAttack` false)
    (set `self.bIsAttacking` true)
    (`KismetSystemLibrary.Delay` (`self.AttackDuration`))
    (set `self.bIsAttacking` false)
    (`KismetSystemLibrary.Delay` (- (`self.CooldownBetweenAttacks`) (`self.AttackDuration`)))
    (set `self.bCanAttack` true)))

(fn `UserConstructionScript`)