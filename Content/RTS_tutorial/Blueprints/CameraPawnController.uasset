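; RTS player controller that drives the camera pawn, unit selection and orders, and building placement.
; Input axes, screen edges and gated mouse panning move or rotate the camera, with speed scaled by spring-arm zoom.
; Left mouse sets selection flags and highlights selected AI characters; right mouse orders them to the cursor hit.
; BeginPlay spawns the construction manager, ghost building and HUD; in build mode the ghost follows the cursor and clicks queue construction.
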(event `InputAction|zoomIn`
  (params (Key :type "Key Structure" :default "AnyKey"))
  (bind _springarm (`/Game/RTS_tutorial/Blueprints/CameraPawn.SpringArm` (`self.CameraPawnRef`)))
  ;[0.1952 1 0.08493] Camera movement
  ;;[0.09543 0.1731 1] My tryin to zoom in
  (:`Pressed`
    (set `SpringArmComponent.TargetArmLength` (`KismetMathLibrary.FClamp` (- (`SpringArmComponent.TargetArmLength` _springarm) 120.0) (`self.MinZoom`) (`self.MaxZoom`)) _springarm)))

(event `InputAxis|MoveForward`
  (params (AxisValue :type "Float (single-precision)"))
  ;[0.1952 1 0.08493] Camera movement
  ;;[1 1 1] movement x
  (if (not false)
    (`self.K2_SetActorTransform` (`self.CameraPawnRef`) (`KismetMathLibrary.MakeTransform` (`KismetMathLibrary.MakeVector` (.x (.location (`self.MovementX` AxisValue (`self.MovementSpeedCalculation`) (`self.FastMoveMultiplier`) (`self.CameraPawnRef`)))) (.y (.location (`self.MovementX` AxisValue (`self.MovementSpeedCalculation`) (`self.FastMoveMultiplier`) (`self.CameraPawnRef`)))) 100.0) (.rotation (`self.MovementX` AxisValue (`self.MovementSpeedCalculation`) (`self.FastMoveMultiplier`) (`self.CameraPawnRef`))) (.scale (`self.MovementX` AxisValue (`self.MovementSpeedCalculation`) (`self.FastMoveMultiplier`) (`self.CameraPawnRef`)))) false false)))

(event `InputAction|zoomOut`
  (params (Key :type "Key Structure" :default "AnyKey"))
  (bind _springarm (`/Game/RTS_tutorial/Blueprints/CameraPawn.SpringArm` (`self.CameraPawnRef`)))
  ;[0.1952 1 0.08493] Camera movement
  ;;[0.1703 0.2932 1] My tryin to zoom out
  (:`Pressed`
    (set `SpringArmComponent.TargetArmLength` (`KismetMathLibrary.FClamp` (- (`SpringArmComponent.TargetArmLength` _springarm) -120.0) (`self.MinZoom`) (`self.MaxZoom`)) _springarm)))

(event `InputAxis|MoveRight`
  (params (AxisValue :type "Float (single-precision)"))
  ;[0.1952 1 0.08493] Camera movement
  ;;[1 1 1] movement z
  (if (not false)
    (`self.K2_SetActorTransform` (`self.CameraPawnRef`) (`self.MovementY` AxisValue (`self.MovementSpeedCalculation`) (`self.FastMoveMultiplier`) (`self.CameraPawnRef`)) false false)))

(event `Key|LeftMouseButton`
  (params (Key :type "Key Structure" :default "AnyKey"))
  ;[1 1 1] left mouse buttton
  (:`Pressed`
    (if (`self.bBuildModeActive`)
      (bind _constructionstruct (`/Game/RTS_tutorial/Blueprints/Buildings/GhostBuilding_BP.GetConstructionStruct` (`self.GhostBuildingRef`)))
      (`/Game/RTS_tutorial/Blueprints/Construction/ConstructionManager_BP.QueueConstruction` (`self.ConstructionManagerRef`) _constructionstruct)
      (`/Game/RTS_tutorial/Blueprints/Buildings/GhostBuilding_BP.KillGhost` (`self.GhostBuildingRef`))
      (else
        (set `self.bSelectionRecActive` true)
        (set `self.b1stPointSet` true))))
  (:`Released`
    (set `self.b1stPointSet` false)
    (set `self.bSelectionRecActive` false)
    (for _array_element (`self.AiCharacters`)
      (bind _asai_character_bp (cast `/Game/RTS_tutorial/Blueprints/AiCharacter_BP` _array_element))
      (if (== (`KismetArrayLibrary.Array_Find` (`self.SelectedActors`) _array_element) -1)
        (bind _mesh (`Character.Mesh` _asai_character_bp))
        (`PrimitiveComponent.SetMaterial` _mesh 0 "/Game/Mannequin/Character/Materials/M_UE4Man_Body.M_UE4Man_Body")
        (`/Game/RTS_tutorial/Blueprints/AiCharacter_BP.HandleSelection` _asai_character_bp false)
        (else
          (`PrimitiveComponent.SetMaterial` _mesh 0 "/Game/StarterContent/Materials/M_Water_Lake.M_Water_Lake")
          (`/Game/RTS_tutorial/Blueprints/AiCharacter_BP.HandleSelection` _asai_character_bp true))))
    (`self.OnSelected`)))

(event `InputAction|panReset`
  (params (Key :type "Key Structure" :default "AnyKey"))
  ;[0.1952 1 0.08493] Camera movement
  ;;[1 1 1] panReset
  (:`Pressed`
    (`self.K2_SetActorRotation` (`self.CameraPawnRef`) (`KismetMathLibrary.MakeRotator` 0.0) false)))

(event `InputAxisKey|MouseX`
  (params (AxisValue :type "Float (single-precision)"))
  ;[0.1952 1 0.08493] Camera movement
  ;;[1 1 1] pan X
  (`/Engine/EditorBlueprintResources/StandardMacros.Gate` true :!label _label
    (:`Exit`
      (`self.K2_SetActorRotation` (`self.CameraPawnRef`) (`KismetMathLibrary.MakeRotator` (.roll (`self.K2_GetActorRotation` (`self.CameraPawnRef`))) (.pitch (`self.K2_GetActorRotation` (`self.CameraPawnRef`))) (+ (.yaw (`self.K2_GetActorRotation` (`self.CameraPawnRef`))) (* (`self.PanSensitivity`) AxisValue))) false))))

(event `InputAction|pan`
  (params (Key :type "Key Structure" :default "AnyKey"))
  ;[0.1952 1 0.08493] Camera movement
  ;;[1 1 1] pan X
  (:`Pressed`
    (set `self.bDisableCamNav` true)
    (goto _label :!via `Open`))
  (:`Released`
    (set `self.bDisableCamNav` false)
    (goto _label :!via `Close`)))

(event `InputAction|ZoomReset`
  (params (Key :type "Key Structure" :default "AnyKey"))
  ;[0.1952 1 0.08493] Camera movement
  ;;[1 1 1] Zoom reset
  (:`Pressed`
    (set `SpringArmComponent.TargetArmLength` 1500.0 (`/Game/RTS_tutorial/Blueprints/CameraPawn.SpringArm` (`self.CameraPawnRef`)))))

(event `InputAxisKey|MouseY`
  (params (AxisValue :type "Float (single-precision)"))
  ;[0.1952 1 0.08493] Camera movement
  ;;[1 1 1] pan Y
  (`/Engine/EditorBlueprintResources/StandardMacros.Gate` true :!label _label_2
    (:`Exit`
      (`self.K2_SetActorRotation` (`self.CameraPawnRef`) (`KismetMathLibrary.MakeRotator` (.roll (`self.K2_GetActorRotation` (`self.CameraPawnRef`))) (`KismetMathLibrary.FClamp` (+ (.pitch (`self.K2_GetActorRotation` (`self.CameraPawnRef`))) (* (`self.PanSensitivity`) AxisValue)) -15.0 45.0) (.yaw (`self.K2_GetActorRotation` (`self.CameraPawnRef`)))) false))))

(event `InputAction|pan`
  (params (Key :type "Key Structure" :default "AnyKey"))
  ;[0.1952 1 0.08493] Camera movement
  ;;[1 1 1] pan Y
  (:`Pressed`
    (set `self.bDisableCamNav` true)
    (goto _label_2 :!via `Open`))
  (:`Released`
    (set `self.bDisableCamNav` false)
    (goto _label_2 :!via `Close`)))

(event `Key|RightMouseButton`
  (params (Key :type "Key Structure" :default "AnyKey"))
  ;[1 1 1] Right mouse button: simple move selected actors
  (:`Pressed`
    (for _array_element (`self.SelectedActors`)
      (`NavigationSystem.SimpleMoveToLocation` (`AIBlueprintHelperLibrary.GetAIController` _array_element) (`.Location` (`GameplayStatics.BreakHitResult` (`self.GetHitResultUnderCursorByChannel` (`GameplayStatics.GetPlayerController` 0) "TraceTypeQuery1" true)))))))

(event `InputAxisKey|MouseY`
  (params (AxisValue :type "Float (single-precision)"))
  (bind _movesensitivity (`self.MovementSpeedCalculation`))
  (bind (_locationx _locationy) (`self.GetMousePosition`))
  (bind _fastmovemultiplier (`self.FastMoveMultiplier`))
  (bind _camerapawnref (`self.CameraPawnRef`))
  (bind (_x _y) (`KismetMathLibrary.BreakVector2D` (`WidgetLayoutLibrary.GetViewportSize`)))
  ;[0.1952 1 0.08493] Camera movement
  ;;[1 1 1] Screen edge movement X
  (if (`self.bDisableCamNav`)
    _
    (elif (>= (/ _locationy _y) 0.975)
      (`self.K2_SetActorTransform` (`self.CameraPawnRef`) (`self.MovementX` -1.0 _movesensitivity _fastmovemultiplier _camerapawnref) false false)
      (elif (<= (/ _locationy _y) 0.025)
        (`self.K2_SetActorTransform` (`self.CameraPawnRef`) (`self.MovementX` 1.0 _movesensitivity _fastmovemultiplier _camerapawnref) false false)))))

(event `self.ReceiveBeginPlay`
  (bind _returnvalue (`KismetMathLibrary.MakeTransform` (0.0 0.0 0.0)))
  ;[1 1 1] begin play
  (`|ExecutionSequence`
    (:`then_0`
      (`self.ReferenceCasts`))
    (:`then_1`
      (bind _returnvalue_2 (`|SpawnActorFromClass` "/Game/RTS_tutorial/Blueprints/Construction/ConstructionManager_BP.ConstructionManager_BP_C" _returnvalue "AlwaysSpawn" "OverrideRootScale" null null))
      (set `self.ConstructionManagerRef` _returnvalue_2))
    (:`then_2`
      (bind _returnvalue_3 (`|SpawnActorFromClass` "/Game/RTS_tutorial/Blueprints/Buildings/GhostBuilding_BP.GhostBuilding_BP_C" _returnvalue "AlwaysSpawn" "OverrideRootScale" null self null))
      (set `self.GhostBuildingRef` _returnvalue_3))
    (:`then_3`
      (`WidgetBlueprintLibrary.SetInputMode_GameAndUIEx` self null "LockAlways" false)
      (`self.CreateHUDs`)
      (`UserWidget.AddToViewport` (`self.MainHUD_Ref`) 0))
    (:`then_4`
      (bind _outactors (`GameplayStatics.GetAllActorsOfClass` "/Game/RTS_tutorial/Blueprints/AiCharacter_BP.AiCharacter_BP_C"))
      (set `self.AiCharacters` _outactors))))

(event `InputAxisKey|MouseX`
  (params (AxisValue :type "Float (single-precision)"))
  (bind _movesensitivity (`self.MovementSpeedCalculation`))
  (bind _locationx (`self.GetMousePosition`))
  (bind _fastmovemultiplier (`self.FastMoveMultiplier`))
  (bind _camerapawnref (`self.CameraPawnRef`))
  (bind _x (`KismetMathLibrary.BreakVector2D` (`WidgetLayoutLibrary.GetViewportSize`)))
  ;[0.1952 1 0.08493] Camera movement
  ;;[1 1 1] Screen edge movement Y
  (if (`self.bDisableCamNav`)
    _
    (elif (>= (/ _locationx _x) 0.975)
      (`self.K2_SetActorTransform` (`self.CameraPawnRef`) (`self.MovementY` 1.0 _movesensitivity _fastmovemultiplier _camerapawnref) false false)
      (elif (<= (/ _locationx _x) 0.025)
        (`self.K2_SetActorTransform` (`self.CameraPawnRef`) (`self.MovementY` -1.0 _movesensitivity _fastmovemultiplier _camerapawnref) false false)))))

(event `self.ReceiveTick`
  (params (DeltaSeconds :type "Float (single-precision)"))
  ;[1 1 1] event tick
  (if (`self.bBuildModeActive`)
    (if (!= (`self.GhostBuildingRef`) null)
      (`/Game/RTS_tutorial/Blueprints/Buildings/GhostBuilding_BP.SetCursorPosition` (`self.GhostBuildingRef`) (`/Game/RTS_tutorial/Libraries/FunctionLibrary.SetCursorWorldPosition` self (`self.SetSightDistance`))))))

(event `InputAction|Deselect`
  (params (Key :type "Key Structure" :default "AnyKey"))
  ;[1 1 1] deselect (right mouse button cancels building)
  (:`Pressed`
    (if (`self.bBuildModeActive`)
      (`/Game/RTS_tutorial/Blueprints/Buildings/GhostBuilding_BP.KillGhost` (`self.GhostBuildingRef`))
      (set `self.bBuildModeActive` false))))

(fn `MovementSpeedCalculation`
  (returns (MoveSensitivity :type "Float (double-precision)"))
  (return (`KismetMathLibrary.FClamp` (/ (`SpringArmComponent.TargetArmLength` (`/Game/RTS_tutorial/Blueprints/CameraPawn.SpringArm` (`self.CameraPawnRef`))) 50.0) 5.0 30.0)))

(fn `MoveToHitByUE4`
  (params (Hit :type "HitResult Structure (by ref)"))
  (bind (_bblockinghit _binitialoverlap _time _location) (`GameplayStatics.BreakHitResult` Hit))
  (if (>= (`KismetMathLibrary.VSize` (- (`self.K2_GetActorLocation` (`self.K2_GetPawn`)) _location)) (`self.MinClickDistance`))
    (`NavigationSystem.SimpleMoveToLocation` self _location) ; Send the destination point to the character
  ))

(fn `SetCallendar`
  (params (Date :type "Array of Integer (by ref)"))
  (returns (Success :type Boolean))
  (return false))

(fn `SetClock`
  (params (Time :type "Array of Integer (by ref)"))
  (returns (Success :type Boolean))
  (return false))

(fn `SetSightDistance`
  (returns (SightDistance :type "Float (double-precision)"))
  (return (+ (`self.SightDistance`) (`SpringArmComponent.TargetArmLength` (`/Game/RTS_tutorial/Blueprints/CameraPawn.SpringArm` (`self.CameraPawnRef`))))))

(fn `UserConstructionScript`)