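; Ghost building actor for the RTS build mode, previewing a building's mesh at the grid-snapped cursor position.
; ConstructBuilding briefly spawns the chosen building to read its mesh and construction proxy, restarts the ghost with them, then destroys it.
; Spawn and kill toggle the controller's build mode and a Tick gate that drives snapped movement.
; GetConstructionStruct packages class, proxy, transform and mesh as construction data.
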(event `OnSpawn`
  (params (DisplayMesh :type "StaticMesh Object Reference") (BuildingClass :type "/Game/RTS_tutorial/Blueprints/Buildings/BuildingMaster_BP Class Reference") (ConstructionProxy :type "/Game/RTS_tutorial/Blueprints/Construction/ConstructionProxy_BP Class Reference"))
  ;[1 1 1] OnSpawn Ghost
  (if (not (`self.IsActive`))
    (set `self.BuildingClass` BuildingClass)
    (set `self.ConstructionProxy` ConstructionProxy)
    (set `self.DisplayMesh` DisplayMesh)
    (set `self.IsActive` true)
    (set `/Game/RTS_tutorial/Blueprints/CameraPawnController.bBuildModeActive` true (`self.ControllerRef`))
    (`StaticMeshComponent.SetStaticMesh` (`self.GhostBuilding_Mesh`) (`self.DisplayMesh`))
    (`self.OpenTickGate`)))

(event `KillGhost`
  ;[1 1 1] kill
  (set `self.BuildingClass` null)
  (set `self.ConstructionProxy` null)
  (`self.CloseTickGate`)
  (set `self.DisplayMesh` null)
  (set `self.IsActive` false)
  (set `/Game/RTS_tutorial/Blueprints/CameraPawnController.bBuildModeActive` false (`self.ControllerRef`))
  (`StaticMeshComponent.SetStaticMesh` (`self.GhostBuilding_Mesh`) (`self.DisplayMesh`)))

(event `/Game/RTS_tutorial/Interfaces/I_HUD.ConstructBuilding`
  (params (MainBuilding :type "/Game/RTS_tutorial/Blueprints/Buildings/BuildingMaster_BP Class Reference"))
  (bind _returnvalue (`|SpawnActorFromClass` MainBuilding (`KismetMathLibrary.MakeTransform` (0.0 0.0 15.0)) "Undefined" "OverrideRootScale" null (`self.ControllerRef`) null))
  (`|ExecutionSequence`
    (:`then_0`
      (bind _asbuilding_master_bp (castclass `/Game/RTS_tutorial/Blueprints/Buildings/BuildingMaster_BP` MainBuilding))
      (`self.KillGhost`)
      (`self.OnSpawn` (`/Game/RTS_tutorial/Blueprints/Buildings/BuildingMaster_BP.DisplayMesh` _returnvalue) _asbuilding_master_bp (`/Game/RTS_tutorial/Blueprints/Buildings/BuildingMaster_BP.ConstructionProxy` _returnvalue)))
    (:`then_1`
      (`self.K2_DestroyActor` _returnvalue))))

(event `self.ReceiveTick`
  (params (DeltaSeconds :type "Float (single-precision)"))
  (`/Engine/EditorBlueprintResources/StandardMacros.Gate` true :!label _label
    (:`Exit`
      (`self.K2_SetActorLocation` self (`self.SetGridSnapVector`) false false))))

(event `OpenTickGate`
  (goto _label :!via `Open`))

(event `CloseTickGate`
  (goto _label :!via `Close`))

(fn `GetConstructionStruct`
  (returns (ConstructionStruct :type "/Game/RTS_tutorial/Structs/Construction_Struct Structure"))
  (return (make `/Game/RTS_tutorial/Structs/Construction_Struct` (`self.BuildingClass`) (`self.ConstructionProxy`) (`KismetMathLibrary.MakeTransform` (`self.K2_GetActorLocation`) (`self.K2_GetActorRotation`)) (`self.DisplayMesh`) 1.0)))

(fn `SetCallendar`
  (params (Date :type "Array of Integer (by ref)"))
  (returns (Success :type Boolean))
  (return false))

(fn `SetClock`
  (params (Time :type "Array of Integer (by ref)"))
  (returns (Success :type Boolean))
  (return false))

(fn `SetCursorPosition`
  (params (CursorLocation :type "Vector Structure"))
  (set `self.CursorWorldPosition` CursorLocation)
  (return))

(fn `SetGridSnapVector`
  (returns (GridSnap :type "Vector Structure"))
  (bind (_cursorworldposition_x _cursorworldposition_y _cursorworldposition_z) (`KismetMathLibrary.BreakVector` (`self.CursorWorldPosition`)))
  (bind _gridsize (`self.GridSize`))
  (return (`KismetMathLibrary.MakeVector` (`/Game/RTS_tutorial/Libraries/FunctionLibrary.GridSnap` _cursorworldposition_x _gridsize) (`/Game/RTS_tutorial/Libraries/FunctionLibrary.GridSnap` _cursorworldposition_y _gridsize) (`/Game/RTS_tutorial/Libraries/FunctionLibrary.GridSnap` _cursorworldposition_z _gridsize))))

(fn `UserConstructionScript`)